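; BP_SleepDummy is a dummy actor that repeatedly fires BP_SleepProjectile, apparently as a test source for sleep shots.
; A looping half-second timer started on BeginPlay calls SpawnProjectile, which spawns with the actor's rotation and scale and sets velocity along negative local X.
; The spawn offset multiplies the forward vector component-wise by an X-only vector, so it shifts only along world X.
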(event `self.ReceiveBeginPlay`
  (`KismetSystemLibrary.K2_SetTimer` null "SpawnProjectile" 0.5 true))

(fn `SpawnProjectile`
  (bind _returnvalue (`|SpawnActorFromClass` "/Game/OliveWatch/AbilitySystem/Abilities/GunFire/BP_SleepProjectile.BP_SleepProjectile_C" (`KismetMathLibrary.MakeTransform` (+ (.location (`self.GetTransform`)) (* (`self.GetActorForwardVector`) (-200.0 0.0 0.0))) (.rotation (`self.GetTransform`)) (.scale (`self.GetTransform`))) "Undefined" "MultiplyWithRoot" null (struct) null))
  (`ProjectileMovementComponent.SetVelocityInLocalSpace` (`OWProjectile.ProjectileMovement` _returnvalue) (-3000.0 0.0 0.0)))

(fn `UserConstructionScript`)